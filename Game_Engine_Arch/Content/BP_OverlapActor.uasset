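; BP_OverlapActor is a randomly placed goal object that ends the game when the player hits it.
; On BeginPlay it moves to a random X/Y location within configurable spawn bounds at a set height.
; A Sphere overlap by the player prints a debug message, while a Cube hit by the player opens the main menu level and prints a win message.
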(event OnComponentBeginOverlap(Sphere)
  (params (OverlappedComponent :type Primitive%20Component%20Object%20Reference) (OtherActor :type Actor%20Object%20Reference) (OtherComp :type Primitive%20Component%20Object%20Reference) (OtherBodyIndex :type Integer) (bFromSweep :type Boolean) (SweepResult :type Hit%20Result%20Structure%20%28by%20ref%29))
  (if (== OtherActor (Game|GetPlayerCharacter 0))
    (Development|PrintString "Overlapping")))

(event OnComponentHit(Cube)
  (params (HitComponent :type Primitive%20Component%20Object%20Reference) (OtherActor :type Actor%20Object%20Reference) (OtherComp :type Primitive%20Component%20Object%20Reference) (NormalImpulse :type Vector :default "0, 0, 0") (Hit :type Hit%20Result%20Structure%20%28by%20ref%29))
  (if (== OtherActor (Game|GetPlayerCharacter 0))
    (Game|OpenLevel(byName) "MainMenuLevel")
    (Development|PrintString "You Won!")))

(event EventBeginPlay
  (Transformation|SetActorLocation (Math|Vector|MakeVector (Math|Random|RandomFloatinRange (Variables|Default|GetMinSpawnX) (Variables|Default|GetMaxSpawnX)) (Math|Random|RandomFloatinRange (Variables|Default|GetMinSpawnY) (Variables|Default|GetMaxSpawnY)) (Variables|Default|GetSpawnZ)) false false))

(event Collision|EventActorBeginOverlap
  (params (OtherActor :type Actor%20Object%20Reference)))

(event EventTick
  (params (DeltaSeconds :type Float%20%28single-precision%29)))

(fn ConstructionScript)